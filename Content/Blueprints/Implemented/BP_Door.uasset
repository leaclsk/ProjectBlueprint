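; BP_Door is an interactable double door that swings two mesh leaves open and closed.
; On Interaction, if CanOpen is set, a FlipFlop alternately plays and reverses a Timeline.
; The Timeline's track, scaled by RotationAngle, yaws the two leaves in opposite directions.
; BeginPlay sets the Timeline play rate to the inverse of Duration, so that variable controls the swing time.
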(event `self.ReceiveBeginPlay`
  (`TimelineComponent.SetPlayRate` (`self.Timeline`) (/ 1.0 (`self.Duration`))))

(event `/Game/Blueprints/Implemented/BPI_Interaction.Interaction`
  (if (`self.CanOpen`)
    (`/Engine/EditorBlueprintResources/StandardMacros.FlipFlop`
      (:`A`
        (bind (_direction _newtrack_0) (`Timeline|Timeline` :!label _label)
          (:`Update`
            (bind _returnvalue (* _newtrack_0 (`self.RotationAngle`)))
            (`SceneComponent.K2_SetRelativeRotation` (`self.Door_3_StaticMeshComponent0`) (`KismetMathLibrary.MakeRotator` 0.0 0.0 (* _returnvalue -1.0)) false false)
            (`SceneComponent.K2_SetRelativeRotation` (`self.Door_4_StaticMeshComponent0`) (`KismetMathLibrary.MakeRotator` 0.0 0.0 _returnvalue) false false))))
      (:`B`
        (goto _label :!via `Reverse`)))))

(fn `UserConstructionScript`)