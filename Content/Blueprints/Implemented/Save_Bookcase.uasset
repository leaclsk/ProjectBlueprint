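; Bookcase puzzle actor that slides aside when the correct code is entered through BP_Button actors.
; It gathers all buttons at BeginPlay and counts ButtonPressed calls, while WrongCode zeroes the count and resets every button.
; At the fourth press, EventMove plays a camera shake and a Movement timeline that lerps the root to TargetLocation in X and Y, keeping its height.
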(event `EventMove`
  (bind (_initiallocation_x _initiallocation_y _initiallocation_z) (`KismetMathLibrary.BreakVector` (`self.InitialLocation`)))
  (bind (_targetlocation_x _targetlocation_y) (`KismetMathLibrary.BreakVector` (`self.TargetLocation`)))
  ;[1 1 1] Mouvement de la commode lorsque le bon code est rentré
  (`GameplayStatics.PlayWorldCameraShake` "/Game/Blueprints/Implemented/BP_CameraShake.BP_CameraShake_C" (`SceneComponent.K2_GetComponentLocation` (`self.SharedRoot`)) 0.0 500.0)
  (set `self.InitialLocation` (`SceneComponent.K2_GetComponentLocation` (`self.SharedRoot`)))
  (bind (_direction _movementvalue) (`Timeline|Movement`)
    (:`Update`
      (`SceneComponent.K2_SetWorldLocation` (`self.SharedRoot`) (`KismetMathLibrary.MakeVector` (`KismetMathLibrary.Lerp` _initiallocation_x _targetlocation_x (.x _movementvalue)) (`KismetMathLibrary.Lerp` _initiallocation_y _targetlocation_y (.y _movementvalue)) _initiallocation_z) false false))))

(event `self.ReceiveBeginPlay`
  ;[1 1 1] Récupère les Buttons
  (`GameplayStatics.GetAllActorsOfClass` "/Game/Blueprints/Implemented/BP_Button.BP_Button_C")
  (for _array_element _
    (`KismetArrayLibrary.Array_Add` (`self.AllButton`) _array_element)))

(event `ButtonPressed`
  (bind _result (`/Engine/EditorBlueprintResources/StandardMacros.IncrementInt` (`self.ButtonOrder`))
    (:`  `
      (set `self.ButtonOrder` _result)
      (if (== (`self.ButtonOrder`) 4)
        (`self.EventMove`)))))

(event `WrongCode`
  ;[1 1 1] Mauvais boutton préssé
  (set `self.ButtonOrder` 0)
  (for _array_element (`self.AllButton`)
    (message `/Game/Blueprints/Implemented/BPI_Interaction.ResetAllButton` _array_element)))

(fn `UserConstructionScript`)