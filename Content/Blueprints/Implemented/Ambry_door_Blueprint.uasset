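; Interactable cupboard (ambry) Blueprint with two doors that swing open and closed.
; The Interaction event, gated by CanOpenCommode, uses a FlipFlop to alternate between playing and reversing a Timeline.
; Each Timeline update scales the track by RotationAngle and sets opposite yaws on the two door meshes, with the first held at a 180-degree pitch.
; The construction script and NewFunction are empty.
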(event `/Game/Blueprints/Implemented/BPI_Interaction.Interaction`
  (if (`self.CanOpenCommode`)
    (`/Engine/EditorBlueprintResources/StandardMacros.FlipFlop`
      (:`A`
        (bind (_direction _newtrack_0) (`Timeline|Timeline` :!label _label)
          (:`Update`
            (bind _returnvalue (* _newtrack_0 (`self.Rotation Angle`)))
            (`SceneComponent.K2_SetRelativeRotation` (`self.Ambry_door_StaticMeshComponent1`) (`KismetMathLibrary.MakeRotator` 0.0 180.0 (* _returnvalue -1.0)) false false)
            (`SceneComponent.K2_SetRelativeRotation` (`self.Ambry_door_StaticMeshComponent2`) (`KismetMathLibrary.MakeRotator` 0.0 0.0 _returnvalue) false false))))
      (:`B`
        (goto _label :!via `Reverse`)))))

(fn `NewFunction`)

(fn `UserConstructionScript`)