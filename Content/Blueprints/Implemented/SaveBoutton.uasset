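; Interactable code button for an ordered-sequence puzzle tied to a Bookcase.
; On Interaction, it compares its ButtonIndex to the Bookcase's ButtonOrder, then reports either a correct press or a wrong code to that Bookcase.
; The Bookcase handles the consequences; the button itself only prints feedback messages, including in its ResetAllButton event, which performs no actual reset.
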(event `self.ResetAllButton`
  ;[1 1 1] Mauvais boutton pressé
  (`KismetSystemLibrary.PrintString` "Mauvais code rentré, recommencez"))

(event `self.Interaction`
  (bind _bookcase (`self.Bookcase`))
  ;[1 1 1] Vérifie que le bon boutton est pressé en comparant son index avec ButtonOrder. Lorsque c'est le bon code, lance le mouvement de la commode, lorsqu'un mouvais bouton est pressé : Reset All Button et
  (if (== (`self.Button_Index`) (`/Game/Blueprints/Implemented/BP_Bookcase.ButtonOrder` (`self.Bookcase`)))
    (`/Game/Blueprints/Implemented/BP_Bookcase.ButtonPressed` _bookcase false)
    (`KismetSystemLibrary.PrintString` "Oui")
    (else
      (`/Game/Blueprints/Implemented/BP_Bookcase.WrongCode` _bookcase)
      (`KismetSystemLibrary.PrintString` "Mauvais code rentré, recommencez"))))

(fn `UserConstructionScript`)