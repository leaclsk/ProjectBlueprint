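; Bookcase puzzle piece that slides to a target location when a four-button code is entered in the correct order.
; ButtonPressed tallies inputs and correctly ordered presses, then triggers either the move or a failure after four inputs.
; EventMove plays a camera shake and uses a timeline to lerp the root's X and Y, keeping its height.
; WrongCode prints a French retry message and resets both counters.
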(event `EventMove`
  (bind (_initiallocation_x _initiallocation_y _initiallocation_z) (`KismetMathLibrary.BreakVector` (`self.InitialLocation`)))
  (bind (_targetlocation_x _targetlocation_y) (`KismetMathLibrary.BreakVector` (`self.TargetLocation`)))
  ;[1 1 1] Mouvement de la commode lorsque le bon code est rentré
  (`GameplayStatics.PlayWorldCameraShake` "/Game/Blueprints/Implemented/BP_CameraShake.BP_CameraShake_C" (`SceneComponent.K2_GetComponentLocation` (`self.SharedRoot`)) 0.0 500.0)
  (set `self.InitialLocation` (`SceneComponent.K2_GetComponentLocation` (`self.SharedRoot`)))
  (bind (_direction _movementvalue) (`Timeline|Movement`)
    (:`Update`
      (`SceneComponent.K2_SetWorldLocation` (`self.SharedRoot`) (`KismetMathLibrary.MakeVector` (`KismetMathLibrary.Lerp` _initiallocation_x _targetlocation_x (.x _movementvalue)) (`KismetMathLibrary.Lerp` _initiallocation_y _targetlocation_y (.y _movementvalue)) _initiallocation_z) false false))))

(event `ButtonPressed`
  (params (GoodOrder :type Boolean))
  (bind _result (`/Engine/EditorBlueprintResources/StandardMacros.IncrementInt` (`self.Nombre_Input`))
    (:`  `
      (set `self.Nombre_Input` _result)
      (if GoodOrder
        (bind _result_2 (`/Engine/EditorBlueprintResources/StandardMacros.IncrementInt` (`self.ButtonOrder`))
          (:`  `
            (set `self.Nombre_Input` _result_2))))
      (if (== (`self.Nombre_Input`) 4)
        (if (== (`self.ButtonOrder`) 4)
          (`self.EventMove`)
          (else
            (`self.WrongCode`)))))))

(event `WrongCode`
  ;[1 1 1] Mauvais boutton préssé
  (`KismetSystemLibrary.PrintString` "Mauvais code, recommencez.")
  (set `self.Nombre_Input` 0)
  (set `self.ButtonOrder` 0))

(fn `UserConstructionScript`)